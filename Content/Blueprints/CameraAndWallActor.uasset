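; Camera actor for a Crossy Road-style game that becomes the player's view target and scrolls steadily forward along X during gameplay.
; Game mode events toggle movement, pausing it on start, kill and loading screens.
; Tick drives a timed, swept lerp between start and end locations, queuing another constant-speed segment when each finishes.
; When the chicken pawn hops ahead of the camera, a short catch-up lerp replaces the current segment.
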(event Custom|On%20Hop
  (params (CurrentLocation :type Vector))
  (if (> (.x CurrentLocation) (.x (Transformation|GetActorLocation)))
    (CallFunction|UpdateMovement (.x CurrentLocation) 0.25)))

(event Custom|On%20Start%20Screen
  (Variables|Default|SetIsMoving false))

(event Custom|On%20Game%20Play
  (Variables|Default|SetIsMoving true)
  (Development|PrintString "Camera Should Be Moving" true true "(R=0.000000,G=1.000000,B=0.134118,A=1.000000)" 2.0 "Camera"))

(event Custom|On%20Kill%20Screen
  (Variables|Default|SetIsMoving false))

(event Custom|On%20Loading
  (Variables|Default|SetIsMoving false))

(event EventBeginPlay
  (CallFunction|SetUp (delegate Custom|On%20Hop) (delegate Custom|On%20Start%20Screen) (delegate Custom|On%20Game%20Play) (delegate Custom|On%20Kill%20Screen) (delegate Custom|On%20Loading)))

(event EventTick
  (params (DeltaSeconds :type Float%20%28single-precision%29))
  (bind _passed_time (CallFunction|Clock DeltaSeconds))
  (CallFunction|Movement (Variables|Default|GetStart%20Location) (Variables|Default|GetEnd%20Location) _passed_time (Variables|Default|GetMax%20Time))
  (Development|PrintString (Utilities|String|ToString(Vector) (Variables|Default|GetStart%20Location)) true true "(R=0.000000,G=0.660000,B=1.000000,A=1.000000)" 2.0 "Camera")
  (Development|PrintString (Utilities|String|ToString(Vector) (Variables|Default|GetEnd%20Location)) true true "(R=0.000000,G=0.660000,B=1.000000,A=1.000000)" 2.0 "Camera 2"))

(fn ConstructionScript)

(fn SetUpCamera
  (Game|Player|SetViewTargetwithBlend (Game|GetPlayerController 0) self 0.0 "VTBlend_Linear" 0.0 false))

(fn Movement
  (params (Start_Location :type Vector) (End_Location :type Vector) (PassedTime :type Float%20%28double-precision%29) (MaxTime :type Float%20%28double-precision%29))
  (bind _returnvalue (Math|Float|NormalizetoRange PassedTime 0.0 MaxTime))
  (if (Variables|Default|GetIsMoving)
    (if (< _returnvalue 1.0)
      (Transformation|SetActorLocation (Math|Vector|Lerp(Vector) Start_Location End_Location _returnvalue) true false)
      (else
        (CallFunction|ResetMovement)))))

(fn Clock
  (params (Delta%20Seconds :type Float%20%28double-precision%29))
  (if (Variables|Default|GetIsMoving)
    (bind _output_get (Variables|Default|SetPassed_Time (+ Delta%20Seconds (Variables|Default|GetPassed_Time))))
    (return _output_get)))

(fn UpdateMovement
  (params (End%20Delta%20X :type Float%20%28double-precision%29) (Max%20Time :type Float%20%28double-precision%29))
  (Utilities|FlowControl|Sequence
    (:then_0
      (bind _output_get (Variables|Default|SetStart%20Location (Transformation|GetActorLocation))))
    (:then_1
      (Variables|Default|SetEnd%20Location (Math|Vector|MakeVector End%20Delta%20X (.y _output_get) (.z _output_get))))
    (:then_2
      (Variables|Default|SetMax%20Time Max%20Time)
      (Variables|Default|SetPassed_Time 0.0))))

(fn ResetMovement
  (bind _distance (Variables|Default|GetDistance))
  (CallFunction|UpdateMovement (+ _distance (.x (Transformation|GetActorLocation))) (/ _distance 2e+02)))

(fn SetUpEvents
  (params (On%20Start%20Screen :type Delegate%20%28by%20ref%29) (On%20Game%20Play :type Delegate%20%28by%20ref%29) (On%20Kill%20Screen :type Delegate%20%28by%20ref%29) (On%20Loading :type Delegate%20%28by%20ref%29))
  (bind _ascrossy_road_game_mode (Utilities|Casting|CastToCrossyRoad_GameMode (Game|GetGameMode))
    (:then
      (EventDispatchers|BindEventtoOnStartScreen _ascrossy_road_game_mode On%20Start%20Screen)
      (EventDispatchers|BindEventtoOnGamePlay _ascrossy_road_game_mode On%20Game%20Play)
      (EventDispatchers|BindEventtoOnKillScreen _ascrossy_road_game_mode On%20Kill%20Screen)
      (EventDispatchers|BindEventtoOnLoading _ascrossy_road_game_mode On%20Loading))
    (:CastFailed
      (Development|PrintString "Game Mode Base Cast FAILED" true true "(R=1.000000,G=0.057555,B=0.000000,A=1.000000)" 2.0 "ERROR"))))

(fn SetUp
  (params (On%20Hop :type Delegate%20%28by%20ref%29) (On%20Start%20Screen :type Delegate%20%28by%20ref%29) (On%20Game%20Play :type Delegate%20%28by%20ref%29) (On%20Kill%20Screen :type Delegate%20%28by%20ref%29) (On%20Loading :type Delegate%20%28by%20ref%29))
  (bind _returnvalue (Actor|GetActorOfClass "/Game/Blueprints/Chicken_Pawn.Chicken_Pawn_C"))
  (EventDispatchers|BindEventtoOnHop _returnvalue On%20Hop)
  (CallFunction|SetUpCamera)
  (CallFunction|ResetMovement)
  (CallFunction|SetUpEvents On%20Start%20Screen On%20Game%20Play On%20Kill%20Screen On%20Loading))