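; Car actor that picks a random static mesh on construction and drives along its local X axis until it is destroyed.
; Tick applies a swept move scaled by MaxSpeed and delta time, and overlapping an actor tagged "Despawn" destroys it.
; Forward line-trace speed adjustment and random MaxSpeed variation exist only as disconnected logic, so CurrentSpeed has no effect on movement.
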(event EventBeginPlay)

(event Collision|EventActorBeginOverlap
  (params (OtherActor :type Actor%20Object%20Reference))
  (if (Actor|ActorHasTag OtherActor "Despawn")
    (Actor|DestroyActor)))

(event EventTick
  (params (DeltaSeconds :type Float%20%28single-precision%29))
  (Class|Actor|AddActorLocalTransform (Math|Transform|MakeTransform (Math|Vector|MakeVector (* DeltaSeconds (Variables|Default|GetMax_Speed)) 0.0 0.0) "0, 0, 0" "1.000000,1.000000,1.000000") true false))

(fn ConstructionScript
  (Components|StaticMesh|SetStaticMesh (Variables|Default|GetCar_StaticMesh) (.OutItem (Utilities|Array|Random (Variables|Default|GetCar_StaticMeshes)))))

(fn ModifySpeed)