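; Player chicken pawn for a Crossy Road-style game, hopping forward, left or right with timed location and rotation lerps.
; Collider hits send the hop back to its start, while Snap-tagged actors carry the chicken by attachment until its next hop.
; Hits, overlaps and landing checks match Car, Train, Eagle and Water tags to play specific death effects.
; It also swaps screen widgets and cursor visibility on game mode events.
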(event OnComponentHit(Collider)
  (params (HitComponent :type Primitive%20Component%20Object%20Reference) (OtherActor :type Actor%20Object%20Reference) (OtherComp :type Primitive%20Component%20Object%20Reference) (NormalImpulse :type Vector :default "0, 0, 0") (Hit :type Hit%20Result%20Structure%20%28by%20ref%29))
  ;[1 1 1] Handles Collision
  (if (Variables|Default|GetCan%20Snap)
    (Utilities|OnComponentHit(Collider)Macro OtherActor OtherComp)))

(event OnComponentBeginOverlap(Collider)
  (params (OverlappedComponent :type Primitive%20Component%20Object%20Reference) (OtherActor :type Actor%20Object%20Reference) (OtherComp :type Primitive%20Component%20Object%20Reference) (OtherBodyIndex :type Integer) (bFromSweep :type Boolean) (SweepResult :type Hit%20Result%20Structure%20%28by%20ref%29))
  ;[1 1 1] Handles Collision
  (if (not (Variables|Default|GetCan%20Snap))
    (CallFunction|ProcessDeath OtherActor OtherComp)))

(event Custom|On%20Eagle%20Death
  (bind _eagle_audio (Variables|Default|GetEagle_Audio))
  ;[1 1 1] Handle Eagle Animation
  (bind (_direction _eagle_x_location _chicken_z_location) (Timeline|Eagle_Death PlayFromStart)
    (:Update
      (Transformation|SetRelativeLocation (Variables|Default|GetEagle_StaticMesh) (Math|Vector|MakeVector _eagle_x_location 0.0 0.0) false false)
      (Transformation|SetRelativeLocation (Variables|Default|GetChicken_SKM) (Math|Vector|MakeVector 0.0 0.0 _chicken_z_location) false false))
    (:Eagle_SFX
      (Audio|Components|Audio|SetSound _eagle_audio (.OutItem (Utilities|Array|Random (Variables|Default|GetEagle_SFXs))))
      (Audio|Components|Audio|Play _eagle_audio 0.0))))

(event Custom|On%20Hop
  (params (Current%20Location :type Vector)))

(event Custom|On%20Start%20Screen
  ;[1 1 1] Handles UI
  (CallFunction|SetUI "/Game/Blueprints/UI/Start_Screen_UI.Start_Screen_UI_C" true))

(event Custom|On%20Game%20Play
  ;[1 1 1] Handles UI
  (CallFunction|SetUI "/Game/Blueprints/UI/Game_Play_UI.Game_Play_UI_C" false))

(event Custom|On%20Kill%20Screen
  ;[1 1 1] Handles UI
  (CallFunction|SetUI "/Game/Blueprints/UI/Kill_Screen_UI.Kill_Screen_UI_C" true))

(event Custom|On%20Loading
  ;[1 1 1] Handles UI
  (CallFunction|SetUI "/Game/Blueprints/UI/Loading_Screen_UI.Loading_Screen_UI_C" false))

(event EventBeginPlay
  ;[1 1 1] Handles UI
  (CallFunction|SetUpEvents (delegate Custom|On%20Start%20Screen) (delegate Custom|On%20Game%20Play) (delegate Custom|On%20Kill%20Screen) (delegate Custom|On%20Loading))
  (CallFunction|OnStartScreen))

(event Collision|EventActorBeginOverlap
  (params (OtherActor :type Actor%20Object%20Reference))
  ;[1 1 1] Handles Collision
  (if (Variables|Default|GetCan%20Snap)
    (Utilities|ActorBeginOverlapMacro OtherActor)))

(event EventTick
  (params (DeltaSeconds :type Float%20%28single-precision%29))
  ;[1 1 1] Handles Movement
  (if (Variables|Hopping|GetIs_Hopping)
    (if (not (Variables|Default|GetIs%20Dead))
      (CallFunction|ProcessHop DeltaSeconds))))

(event Input|ActionEvents|InputActionHopForward
  (params (Key :type Key%20Structure :default "None"))
  ;[1 1 1] Handles Input
  (:Pressed
    (Utilities|IfNOTDeadThenUnSnap)
    (CallFunction|StartHop "1.000000, 0, 0")
    (Default|CallOnHopForward)))

(event Input|ActionEvents|InputActionHopLeft
  (params (Key :type Key%20Structure :default "None"))
  ;[1 1 1] Handles Input
  (:Pressed
    (Utilities|IfNOTDeadThenUnSnap)
    (CallFunction|StartHop "0,-1.000000, 0")))

(event Input|ActionEvents|InputActionHopRight
  (params (Key :type Key%20Structure :default "None"))
  ;[1 1 1] Handles Input
  (:Pressed
    (Utilities|IfNOTDeadThenUnSnap)
    (CallFunction|StartHop "0,1.000000, 0")))

(fn ConstructionScript)

(fn StartHop
  (params (Directon :type Vector))
  (bind _returnvalue (Transformation|GetActorLocation))
  (bind (_x _y) (Class|KismetMathLibrary|BreakVector3f Directon))
  (bind _chicken_audio (Variables|Default|GetChicken_Audio))
  (if (not (Variables|Hopping|GetIs_Hopping))
    (Variables|Hopping|SetIs_Hopping true)
    (Variables|Hopping|SetStart (Math|Transform|MakeTransform _returnvalue (Variables|/Script/Engine.SceneComponent|GetRelativeRotation (Variables|Default|GetChicken_SKM)) "1.000000,1.000000,1.000000"))
    (Variables|Hopping|SetEnd (Math|Transform|MakeTransform (+ _returnvalue (* Directon (Variables|Hopping|GetHop_Distance))) (Math|Rotator|MakeRotator 0.0 0.0 (Class|KismetMathLibrary|DegAtan2 (* _x -1.0) _y)) "1.000000,1.000000,1.000000"))
    (Components|Animation|PlayAnimation (Variables|Default|GetChicken_SKM) "/Game/Animations/Chicken_Jump_Anim.Chicken_Jump_Anim" false)
    (Audio|Components|Audio|SetSound _chicken_audio (.OutItem (Utilities|Array|Random (Variables|Default|GetHop_SFXs))))
    (Audio|Components|Audio|Play _chicken_audio 0.0)))

(fn ProcessHop
  (params (Delta_Seconds :type Float%20%28double-precision%29))
  (bind _end (Variables|Hopping|GetEnd))
  (bind _max_time (Variables|Time|GetMax%20Time))
  (Utilities|FlowControl|Sequence
    (:then_0
      ;[1 1 1] Times Movement
      (bind _output_get (Variables|Time|SetPassed%20Time (+ Delta_Seconds (Variables|Time|GetPassed%20Time))))
      ;[1 1 1] Stops movement
      (if (>= _output_get _max_time)
        (Variables|Time|SetPassed%20Time 0.0)
        (Variables|Hopping|SetIs_Hopping false)
        (if (Variables|Default|GetCan%20Snap)
          (Transformation|SetActorLocation (.location _end) false true) ; Snaps the actor to the end position to avoid float-point error bugs is not triggered when the player snaps to a log
        )
        (Default|CallOnHop (.location _end))
        (CallFunction|TrytoKill)
        (return)))
    (:then_1
      (if (Variables|Default|GetCan%20Snap)
        ;[1 1 1] Rotats Chicken_SKM
        (Transformation|SetRelativeRotation (Variables|Default|GetChicken_SKM) (Math|Rotator|Lerp(Rotator) (.rotation (Variables|Hopping|GetStart)) (.rotation (Variables|Hopping|GetEnd)) (Math|Float|NormalizetoRange _output_get 0.0 _max_time) true) false false)
        ;[1 1 1] Lerps Pawn
        (Transformation|SetActorLocation (Math|Vector|Lerp(Vector) (.location (Variables|Hopping|GetStart)) (.location (Variables|Hopping|GetEnd)) (Math|Float|NormalizetoRange _output_get 0.0 _max_time)) true false)
        (else
          ;[1 1 1] Handles when the character snaps to a log
          (Transformation|SetRelativeRotation (Variables|Default|GetChicken_SKM) (.rotation (Variables|Hopping|GetEnd)) false false))))))

(fn ProcessDeath
  (params (Other_Actor :type Actor%20Object%20Reference) (Other_Component :type Actor%20Component%20Object%20Reference))
  (bind _chicken_audio (Variables|Default|GetChicken_Audio))
  (LocalVariables|SetOther%20Actor Other_Actor)
  (if (not (Variables|Default|GetIs%20Dead))
    (for _array_element (Variables|/Script/Engine.Actor|GetTags Other_Actor)
      (switch name _array_element
        (:Car
          (if (Utilities|AreActorXCordsEqual (LocalVariables|GetOther%20Actor))
            (Development|PrintString "Play Splat Death Animation" false true "(R=1.000000,G=0.000000,B=0.215297,A=1.000000)" 2.0 "Animation")
            (Components|Animation|PlayAnimation (Variables|Default|GetChicken_SKM) "/Game/Animations/Chicken_Death_Splat_Anim.Chicken_Death_Splat_Anim" false)
            (CallFunction|SnaptoWorld (LocalVariables|GetOther%20Actor))
            (else
              (Development|PrintString "Play Squish Death Animation" false true "(R=1.000000,G=0.000000,B=0.215297,A=1.000000)" 2.0 "Animation")
              (Components|Animation|PlayAnimation (Variables|Default|GetChicken_SKM) "/Game/Animations/Chicken_Death_Squish_Anim.Chicken_Death_Squish_Anim" false)))
          (Variables|Default|SetIs%20Dead true :!label _label)
          (Audio|Components|Audio|SetVolumeMultiplier _chicken_audio 8.0 :!class /Script/Engine.AudioComponent)
          (Audio|Components|Audio|SetSound _chicken_audio (.OutItem (Utilities|Array|Random (Variables|Default|GetDeath_SFXs))))
          (Audio|Components|Audio|Play _chicken_audio 0.0)
          (Default|CallOnDeath)
          (return))
        (:Train
          (Development|PrintString "Play Feather Explosion Death Animation" false true "(R=1.000000,G=0.000000,B=0.215297,A=1.000000)" 2.0 "Animation")
          (Components|Animation|PlayAnimation (Variables|Default|GetChicken_SKM) "/Game/Animations/Chicken_Death_Squish_Anim.Chicken_Death_Squish_Anim" false)
          (Components|Activation|Activate (Variables|Default|GetChicken_Train_Death_NiagaraSystem) false)
          (goto _label))
        (:Eagle
          (Development|PrintString "Play Eagle Death Animation" false true "(R=1.000000,G=0.000000,B=0.215297,A=1.000000)" 2.0 "Animation")
          (Components|Animation|PlayAnimation (Variables|Default|GetChicken_SKM) "/Game/Animations/Chicken_Death_Explode_Anim.Chicken_Death_Explode_Anim" false)
          (CallFunction|OnEagleDeath)
          (goto _label))
        (:Water
          (if (Variables|Default|GetCan%20Snap)
            (Development|PrintString "Play Drowning Death Animation" false true "(R=1.000000,G=0.000000,B=0.215297,A=1.000000)" 2.0 "Animation")
            (Components|Animation|PlayAnimation (Variables|Default|GetChicken_SKM) "/Game/Animations/Chicken_Death_Squish_Anim.Chicken_Death_Squish_Anim" false)
            (Transformation|SetRelativeLocation (Variables|Default|GetChicken_SKM) "0, 0,-50.000000" false false)
            (Components|Activation|Activate (Variables|Default|GetChicken_Water_Death_NiagaraSystem) false)
            (Audio|Components|Audio|Play (Variables|Default|GetSplash_Audio) 0.0)
            (goto _label)))))
    (if (not (Variables|Default|GetIs%20Dead))
      (for _array_element_2 (Variables|/Script/Engine.ActorComponent|GetComponentTags Other_Component)
        (switch name _array_element_2
          (:Car
            (if (Utilities|AreActorXCordsEqual (LocalVariables|GetOther%20Actor))
              (Development|PrintString "Play Splat Death Animation" false true "(R=1.000000,G=0.000000,B=0.215297,A=1.000000)" 2.0 "Animation")
              (Components|Animation|PlayAnimation (Variables|Default|GetChicken_SKM) "/Game/Animations/Chicken_Death_Splat_Anim.Chicken_Death_Splat_Anim" false)
              (CallFunction|SnaptoWorld (LocalVariables|GetOther%20Actor))
              (else
                (Development|PrintString "Play Squish Death Animation" false true "(R=1.000000,G=0.000000,B=0.215297,A=1.000000)" 2.0 "Animation")
                (Components|Animation|PlayAnimation (Variables|Default|GetChicken_SKM) "/Game/Animations/Chicken_Death_Squish_Anim.Chicken_Death_Squish_Anim" false)))
            (Variables|Default|SetIs%20Dead true :!label _label_2)
            (Audio|Components|Audio|SetVolumeMultiplier _chicken_audio 8.0 :!class /Script/Engine.AudioComponent)
            (Audio|Components|Audio|SetSound _chicken_audio (.OutItem (Utilities|Array|Random (Variables|Default|GetDeath_SFXs))))
            (Audio|Components|Audio|Play _chicken_audio 0.0)
            (Default|CallOnDeath)
            (return))
          (:Train
            (Development|PrintString "Play Feather Explosion Death Animation" false true "(R=1.000000,G=0.000000,B=0.215297,A=1.000000)" 2.0 "Animation")
            (Components|Animation|PlayAnimation (Variables|Default|GetChicken_SKM) "/Game/Animations/Chicken_Death_Squish_Anim.Chicken_Death_Squish_Anim" false)
            (Components|Activation|Activate (Variables|Default|GetChicken_Train_Death_NiagaraSystem) false)
            (goto _label_2))
          (:Eagle
            (Development|PrintString "Play Eagle Death Animation" false true "(R=1.000000,G=0.000000,B=0.215297,A=1.000000)" 2.0 "Animation")
            (Components|Animation|PlayAnimation (Variables|Default|GetChicken_SKM) "/Game/Animations/Chicken_Death_Explode_Anim.Chicken_Death_Explode_Anim" false)
            (CallFunction|OnEagleDeath)
            (goto _label_2))
          (:Water
            (if (Variables|Default|GetCan%20Snap)
              (Development|PrintString "Play Drowning Death Animation" false true "(R=1.000000,G=0.000000,B=0.215297,A=1.000000)" 2.0 "Animation")
              (Components|Animation|PlayAnimation (Variables|Default|GetChicken_SKM) "/Game/Animations/Chicken_Death_Squish_Anim.Chicken_Death_Squish_Anim" false)
              (Transformation|SetRelativeLocation (Variables|Default|GetChicken_SKM) "0, 0,-50.000000" false false)
              (Components|Activation|Activate (Variables|Default|GetChicken_Water_Death_NiagaraSystem) false)
              (Audio|Components|Audio|Play (Variables|Default|GetSplash_Audio) 0.0)
              (goto _label_2))))))))

(fn ProcessWall
  (params (Other%20Actor :type Actor%20Object%20Reference) (Other%20Component :type Actor%20Component%20Object%20Reference))
  (Variables|Hopping|SetEnd (Variables|Hopping|GetStart))
  (Variables|Hopping|SetStart (Math|Transform|MakeTransform (Transformation|GetActorLocation) (Transformation|GetActorRotation) "1.000000,1.000000,1.000000")))

(fn SetUpCamera
  (Game|Player|SetViewTargetwithBlend (Game|GetPlayerController 0) (Variables|References|GetCamera) 0.0 "VTBlend_Linear" 0.0 false))

(fn SetUpEvents
  (params (On%20Start%20Screen :type Delegate%20%28by%20ref%29) (On%20Game%20Play :type Delegate%20%28by%20ref%29) (On%20Kill%20Screen :type Delegate%20%28by%20ref%29) (On%20Loading :type Delegate%20%28by%20ref%29))
  (bind _ascrossy_road_game_mode (Utilities|Casting|CastToCrossyRoad_GameMode (Game|GetGameMode)))
  (EventDispatchers|BindEventtoOnStartScreen _ascrossy_road_game_mode On%20Start%20Screen)
  (EventDispatchers|BindEventtoOnGamePlay _ascrossy_road_game_mode On%20Game%20Play)
  (EventDispatchers|BindEventtoOnKillScreen _ascrossy_road_game_mode On%20Kill%20Screen)
  (EventDispatchers|BindEventtoOnLoading _ascrossy_road_game_mode On%20Loading))

(fn SetUI
  (params (UI%20Widget%20Class :type User%20Widget%20Class%20Reference) (Show%20Mouse :type Boolean))
  (if (Utilities|IsValid (Variables|Default|GetCurren%20UI))
    (Widget|RemovefromParent (Variables|Default|GetCurren%20UI)))
  (bind _returnvalue (UserInterface|CreateWidget UI%20Widget%20Class))
  (bind _output_get (Variables|Default|SetCurren%20UI _returnvalue))
  (UserInterface|Viewport|AddtoViewport _output_get 0)
  (Variables|/Script/Engine.PlayerController|SetbShowMouseCursor (Game|GetPlayerController 0) Show%20Mouse))

(fn TurnOffUI
  (Widget|RemovefromParent (Variables|Default|GetCurren%20UI))
  (Variables|/Script/Engine.PlayerController|SetbShowMouseCursor (Game|GetPlayerController 0) false))

(fn SnaptoWorld
  (params (Other%20Actor :type Actor%20Object%20Reference))
  (CallFunction|UnSnapto)
  (Transformation|AttachActorToActor Other%20Actor "None" "KeepWorld" "KeepWorld" "KeepWorld" false))

(fn UnSnapto
  (Transformation|DetachFromActor "KeepWorld" "KeepWorld" "KeepWorld")
  (Variables|Default|SetCan%20Snap true))

(fn SnaptoTarget
  (params (Other%20Actor :type Actor%20Object%20Reference))
  (if (Variables|Default|GetCan%20Snap)
    (Variables|Default|SetCan%20Snap false)
    (Transformation|DetachFromActor "KeepWorld" "KeepWorld" "KeepWorld")
    (Transformation|AttachActorToActor Other%20Actor "None" "SnapToTarget" "KeepWorld" "KeepWorld" false)))

(fn TrytoKill
  (bind _outactors (Collision|ComponentOverlapActors (Variables|Default|GetCollider) (Transformation|GetActorTransform) (Variables|Default|GetObject%20Types) 0))
  (for _array_element _outactors
    (CallFunction|ProcessDeath _array_element (Variables|Default|GetEagle_StaticMesh))))