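; Game mode for a Crossy Road-style game that runs the start, gameplay, kill and loading screen states and tracks lane score and coins.
; On BeginPlay it binds the Chicken_Pawn's hop, death and forward-hop events to drive state changes, which fire per-state dispatchers, and scoring.
; High score and coin count persist through a SaveGame slot, saved on each coin or new record.
; Tick prints the current state to screen for debugging.
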(event Custom|On%20State%20Update
  (params (New%20State :type Game_States%20Enum :default "NewEnumerator0")))

(event Custom|On%20Hop
  (params (CurrentLocation :type Vector))
  ;[1 1 1] Switching from Start State to Game Play
  (if (Utilities|Enum|Equal(Enum) (Variables|Public|GetCurrentState) "NewEnumerator0")
    (Public|SetCurrentState "NewEnumerator1")))

(event Custom|On%20Death
  ;[1 1 1] Trigging Kill Screen
  (Public|SetCurrentState "NewEnumerator2"))

(event Custom|On%20Chicken%20Hop%20Forward
  ;[1 1 1] Updating Lane Score
  (Private|UpdateLaneScore))

(event EventBeginPlay
  ;[1 1 1] Set Up
  (Public|SetUpEvents (delegate Custom|On%20Hop) (delegate Custom|On%20Death) (delegate Custom|On%20Chicken%20Hop%20Forward))
  (Private|LoadGame))

(event EventTick
  (params (DeltaSeconds :type Float%20%28single-precision%29))
  ;[1 1 1] Printing Current State To Screen
  (Development|PrintString (Utilities|String|EnumtoString (Variables|Public|GetCurrentState)) true true "(R=0.000000,G=0.505208,B=0.008877,A=1.000000)" 2.0 "State"))

(fn ConstructionScript)

(fn SetCurrentState
  (params (NewCurrentState :type Game_States%20Enum :default "NewEnumerator0"))
  (bind _output_get (Variables|Public|SetCurrentState NewCurrentState))
  (CallFunction|OnStateUpdate _output_get)
  (switch Utilities|FlowControl|Switch|SwitchonGame_States _output_get
    (:NewEnumerator0
      (Default|CallOnStartScreen))
    (:NewEnumerator1
      (Default|CallOnGamePlay))
    (:NewEnumerator2
      (Default|CallOnKillScreen))
    (:NewEnumerator3
      (Default|CallOnLoading))))

(fn SetUpEvents
  (params (On%20Hop%20Event :type Delegate%20%28by%20ref%29) (On%20Death%20Event :type Delegate%20%28by%20ref%29) (On%20Hop%20Forward%20Event :type Delegate%20%28by%20ref%29))
  (bind _returnvalue (Actor|GetActorOfClass "/Game/Blueprints/Chicken_Pawn.Chicken_Pawn_C"))
  (EventDispatchers|BindEventtoOnHop _returnvalue On%20Hop%20Event)
  (EventDispatchers|BindEventtoOnDeath _returnvalue On%20Death%20Event)
  (EventDispatchers|BindEventtoOnHopForward _returnvalue On%20Hop%20Forward%20Event)
  (Public|SetCurrentState "NewEnumerator0"))

(fn OnCollectCoin
  (Math|Integer|IncrementInt (Variables|Public|GetCoinCount)
    (:%20%20
      (Private|SaveGame)
      (Audio|Components|Audio|Play (Variables|Default|GetCoin_Audio) 0.0))))

(fn UpdateLaneScore
  (bind _result (Math|Integer|IncrementInt (Variables|Public|GetCurrent_LaneScore))
    (:%20%20
      (Variables|Public|SetCurrent_LaneScore _result)
      (if (> (Variables|Public|GetCurrent_LaneScore) (Variables|Public|GetLane_HighScore))
        (Variables|Public|SetLane_HighScore (Variables|Public|GetCurrent_LaneScore))
        (Private|SaveGame)))))

(fn SaveGame
  (bind _coincount (Variables|Public|GetCoinCount))
  (bind _returnvalue (SaveGame|DoesSaveGameExist (Variables|Private|GetSaveGame_SlotName)))
  (if _returnvalue
    (bind _returnvalue_2 (SaveGame|LoadGamefromSlot (Variables|Private|GetSaveGame_SlotName)))
    (bind _ascrossy_road_save_game (Utilities|Casting|CastToCrossyRoad_SaveGame _returnvalue_2))
    (bind _output_get (Variables|Private|SetGameSaveData _ascrossy_road_save_game))
    (Variables|/Game/Blueprints/CrossyRoad_SaveGame.CrossyRoad_SaveGame_C|SetLane_HighScore _output_get (Variables|Public|GetLane_HighScore))
    (Variables|/Game/Blueprints/CrossyRoad_SaveGame.CrossyRoad_SaveGame_C|SetCoin_Count _output_get _coincount)
    (else
      (bind _returnvalue_3 (SaveGame|CreateSaveGameObject "/Game/Blueprints/CrossyRoad_SaveGame.CrossyRoad_SaveGame_C"))
      (bind _output_get_2 (Variables|Private|SetGameSaveData _returnvalue_3))
      (Variables|/Game/Blueprints/CrossyRoad_SaveGame.CrossyRoad_SaveGame_C|SetLane_HighScore _output_get_2 (Variables|Public|GetLane_HighScore))
      (Variables|/Game/Blueprints/CrossyRoad_SaveGame.CrossyRoad_SaveGame_C|SetCoin_Count _output_get_2 _coincount)))
  (SaveGame|SaveGametoSlot (Variables|Private|GetGameSaveData) (Variables|Private|GetSaveGame_SlotName)))

(fn LoadGame
  (bind _returnvalue (SaveGame|DoesSaveGameExist (Variables|Private|GetSaveGame_SlotName)))
  (if _returnvalue
    (bind _returnvalue_2 (SaveGame|LoadGamefromSlot (Variables|Private|GetSaveGame_SlotName)))
    (bind _ascrossy_road_save_game (Utilities|Casting|CastToCrossyRoad_SaveGame _returnvalue_2))
    (bind _output_get (Variables|Private|SetGameSaveData _ascrossy_road_save_game))
    (Variables|Public|SetLane_HighScore (Variables|/Game/Blueprints/CrossyRoad_SaveGame.CrossyRoad_SaveGame_C|GetLane_HighScore _output_get))
    (Variables|Public|SetCoinCount (Variables|/Game/Blueprints/CrossyRoad_SaveGame.CrossyRoad_SaveGame_C|GetCoin_Count _output_get))
    (else
      (bind _returnvalue_3 (SaveGame|CreateSaveGameObject "/Game/Blueprints/CrossyRoad_SaveGame.CrossyRoad_SaveGame_C"))
      (bind _output_get_2 (Variables|Private|SetGameSaveData _returnvalue_3))
      (Variables|Public|SetLane_HighScore (Variables|/Game/Blueprints/CrossyRoad_SaveGame.CrossyRoad_SaveGame_C|GetLane_HighScore _output_get_2))
      (Variables|Public|SetCoinCount (Variables|/Game/Blueprints/CrossyRoad_SaveGame.CrossyRoad_SaveGame_C|GetCoin_Count _output_get_2)))))

(fn DeleteSaveGame
  (bind _returnvalue (SaveGame|DoesSaveGameExist (Variables|Private|GetSaveGame_SlotName)))
  (if _returnvalue
    (SaveGame|DeleteGameinSlot (Variables|Private|GetSaveGame_SlotName))
    (Private|LoadGame)))