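; Lane actor for a chicken road-crossing game, forming one segment of a lane track that rolls forward as the player advances.
; On construction it applies a random floor material and caches the world transform where the next lane attaches.
; When an actor tagged Player overlaps it, it tells its assigned LaneManager to spawn a random lane and delete the last one.
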(event EventBeginPlay)

(event Collision|EventActorBeginOverlap
  (params (OtherActor :type Actor%20Object%20Reference))
  (Protected|ChickenDetected OtherActor))

(event EventTick
  (params (DeltaSeconds :type Float%20%28single-precision%29)))

(fn ConstructionScript
  (Protected|Generate))

(fn ChickenDetected
  (params (Other%20Actor :type Actor%20Object%20Reference))
  (bind _lane_manager (Variables|Reference|GetLane_Manager))
  (if (Actor|ActorHasTag Other%20Actor "Player")
    (Default|SpawnRandomLane _lane_manager)
    (Default|DeleteLastLane _lane_manager)))

(fn Generate
  (CallFunction|SetFloorMaterial (.OutItem (Utilities|Array|Random (Variables|Public|GetFloorMaterials))))
  (Variables|Public|SetNextLaneWorldSpawnPoint (Transformation|GetWorldTransform (Variables|Default|GetNext_Lane_Spawn_Point))))

(fn SetLaneManager
  (params (New_Lane_Manager :type Lane%20Manager%20Object%20Reference))
  (Variables|Reference|SetLane_Manager New_Lane_Manager))

(fn SetFloorMaterials
  (params (Materials :type Array%20of%20Material%20Object%20References))
  (Variables|Public|SetFloorMaterials Materials))

(fn SetFloorMaterial
  (params (Material :type Material%20Interface%20Object%20Reference))
  (Rendering|Material|SetMaterial (Variables|Default|GetFloor) 0 Material))