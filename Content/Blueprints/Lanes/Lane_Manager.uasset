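; Lane manager actor that builds a procedural chain of lanes, starting from its own transform on BeginPlay.
; It spawns a fixed opening sequence, then random lanes with a one-in-four chance of water.
; Each lane receives a manager reference and supplies the next spawn point, while grass lanes alternate between two floor materials.
; Lanes are tracked in an array, and DeleteLastLane destroys the oldest.
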(event EventBeginPlay
  (Private|SpawnInitialLanes))

(event Collision|EventActorBeginOverlap
  (params (OtherActor :type Actor%20Object%20Reference)))

(event EventTick
  (params (DeltaSeconds :type Float%20%28single-precision%29)))

(fn ConstructionScript)

(fn SpawnRandomLane
  (if (== (Math|Random|RandomIntegerinRange 1 4) 1)
    (bind _returnvalue (Game|SpawnActorfromClass (.OutItem (Utilities|Array|Random (Variables|Public|GetWater_Lanes))) (Variables|Private|GetLaneSpawnTransform) "Undefined" 0 0))
    (CallFunction|SetUpLane _returnvalue)
    (else
      (bind _returnvalue_2 (Game|SpawnActorfromClass (.OutItem (Utilities|Array|Random (Variables|Public|GetLanesToSpawn))) (Variables|Private|GetLaneSpawnTransform) "Undefined" 0 0))
      (bind _aslane (Utilities|Casting|CastToLane _returnvalue_2))
      (CallFunction|SetUpLane _aslane))))

(fn SpawnInitialLanes
  (Variables|Private|SetLaneSpawnTransform (Transformation|GetActorTransform))
  (for _array_element (Variables|/Game/Blueprints/Lanes/Lane_Sequences/Lane_Sequence.Lane_Sequence_C|GetLanes (Variables|Public|GetStart_Lane_Sequence))
    (CallFunction|SpawnExactLane _array_element))
  (for _index (range 0 (Variables|Private|GetInitialAmountOfLanesToSpawn))
    (Public|SpawnRandomLane)))

(fn DeleteLastLane
  (bind _lanes (Variables|Private|GetLanes))
  (Actor|DestroyActor (Utilities|Array|Get(acopy) _lanes))
  (Utilities|Array|RemoveIndex _lanes))

(fn SpawnExactLane
  (params (New%20Lane :type Lane%20Class%20Reference))
  (bind _returnvalue (Game|SpawnActorfromClass New%20Lane (Variables|Private|GetLaneSpawnTransform) "Undefined" 0 0))
  (CallFunction|SetUpLane _returnvalue))

(fn SetUpLane
  (params (NewLane :type Lane%20Object%20Reference))
  (Utilities|FlowControl|Sequence
    (:then_0
      (Utilities|Array|Add (Variables|Private|GetLanes) NewLane)
      (bind _output_get (Variables|Reference|SetLatest_Lane NewLane))
      (Default|SetLaneManager _output_get self)
      (Variables|Private|SetLaneSpawnTransform (Variables|/Game/Blueprints/Lanes/Lane.Lane_C|GetNextLaneWorldSpawnPoint _output_get)))
    (:then_1
      (bind _asgrass_lane (Utilities|Casting|CastToGrass_Lane NewLane))
      (if (Variables|Private|GetGrass_IsColor1)
        (Default|SetFloorMaterial _asgrass_lane (Utilities|Array|Get(acopy) (Variables|/Game/Blueprints/Lanes/Lane.Lane_C|GetFloorMaterials _asgrass_lane)))
        (Variables|Private|SetGrass_IsColor1 false)
        (else
          (Default|SetFloorMaterial _asgrass_lane (Utilities|Array|Get(acopy) (Variables|/Game/Blueprints/Lanes/Lane.Lane_C|GetFloorMaterials _asgrass_lane) 1))
          (Variables|Private|SetGrass_IsColor1 true))))))