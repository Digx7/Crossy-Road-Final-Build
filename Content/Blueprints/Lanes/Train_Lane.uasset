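; Train lane actor that alerts its train signal when a spawn happens on the lane.
; OnSpawn casts the TrainSignal child actor to TrainSignal and fires its EventTrainSpawn.
; The remaining events are disabled stubs, and the construction script only calls the parent.
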(event EventBeginPlay
  (|CallParentFunction) ; This node is disabled and will not be called.\nDrag off pins to build functionality.
)

(event Collision|EventActorBeginOverlap
  (params (OtherActor :type Actor%20Object%20Reference))
  (|CallParentFunction OtherActor) ; This node is disabled and will not be called.\nDrag off pins to build functionality.
)

(event EventTick
  (params (DeltaSeconds :type Float%20%28single-precision%29))
  (|CallParentFunction DeltaSeconds) ; This node is disabled and will not be called.\nDrag off pins to build functionality.
)

(event EventOnSpawn
  (bind _astrain_signal (Utilities|Casting|CastToTrainSignal (Variables|/Script/Engine.ChildActorComponent|GetChildActor (Variables|Default|GetTrainSignal))))
  (Default|EventTrainSpawn _astrain_signal))

(fn ConstructionScript
  (|CallParentFunction))