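; Water lane Blueprint that sets up the kill volumes for a stretch of water among the game's lanes.
; On BeginPlay, after calling its parent, it spawns a Water_Kill_Box at the water point and a Kill_Box at each of the right and left points.
; Each spawn takes its transform from a component on the lane, with only the water box explicitly forced to spawn regardless of collision.
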(event EventBeginPlay
  (|CallParentFunction)
  (Game|SpawnActorfromClass "/Game/Blueprints/Water_Kill_Box.Water_Kill_Box_C" (Transformation|GetWorldTransform (Variables|Default|GetWater_Kill_Box_Point1)) "AlwaysSpawn" 0 0)
  (Game|SpawnActorfromClass "/Game/Blueprints/Kill_Box.Kill_Box_C" (Transformation|GetWorldTransform (Variables|Default|GetKill_Box_Point_R)) "Undefined" 0 0)
  (Game|SpawnActorfromClass "/Game/Blueprints/Kill_Box.Kill_Box_C" (Transformation|GetWorldTransform (Variables|Default|GetKill_Box_Point_L)) "Undefined" 0 0))

(event Collision|EventActorBeginOverlap
  (params (OtherActor :type Actor%20Object%20Reference))
  (|CallParentFunction OtherActor) ; This node is disabled and will not be called.\nDrag off pins to build functionality.
)

(event EventTick
  (params (DeltaSeconds :type Float%20%28single-precision%29))
  (|CallParentFunction DeltaSeconds) ; This node is disabled and will not be called.\nDrag off pins to build functionality.
)

(fn ConstructionScript
  (|CallParentFunction))