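; Train signal actor that sounds and flashes its two lights when its TrainSpawn event fires.
; TrainSpawn starts the signal audio and plays the TrainSignal timeline from the beginning.
; Each timeline update passes the LightsTrack X and Y values to OnTrainSpawn, which shows each point light while its value is above zero.
; The mapping is crossed: X (Light1) drives PointLight2 and Y (Light2) drives PointLight1.
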(event Custom|Event%20Train%20Spawn
  (Audio|Components|Audio|Play (Variables|Default|GetSignal_Audio) 0.0)
  (bind _lights_track (Timeline|TrainSignal PlayFromStart)
    (:Update
      (CallFunction|OnTrainSpawn (.x _lights_track) (.y _lights_track)))))

(event EventBeginPlay)

(event Collision|EventActorBeginOverlap
  (params (OtherActor :type Actor%20Object%20Reference)))

(event EventTick
  (params (DeltaSeconds :type Float%20%28single-precision%29)))

(fn ConstructionScript)

(fn OnTrainSpawn
  (params (Light%201 :type Float%20%28double-precision%29) (Light%202 :type Float%20%28double-precision%29))
  (bind _output_get (Variables|Default|SetLight%201 (> Light%201 0.0)))
  (Rendering|SetVisibility (Variables|Default|GetPointLight_2) _output_get false)
  (bind _output_get_2 (Variables|Default|SetLight%202 (> Light%202 0.0)))
  (Rendering|SetVisibility (Variables|Default|GetPointLight_1) _output_get_2 false))